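; Procedurally builds a descending, side-on grid of mud, gravel and rock blocks with cave gaps, extending it as the player goes deeper.
; BeginPlay seeds Perlin noise and spawns the initial rows; Tick adds 20-row batches whenever the first player drops below a moving Z threshold.
; LineGen mixes noise with randomness against WorldData thresholds, favouring rock and gravel with depth and keeping top rows solid mud.
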(event EventBeginPlay
  (CallFunction|GenNoise)
  (CallFunction|CreateMap)
  (Variables|Default|SetThreshold (+ (- (* (.Y (Math|Vector2D|BreakVector2D (Variables|Default|GetSize))) 2e+02) (.z (Transformation|GetActorLocation))) 1e+03)))

(event EventTick
  (params (DeltaSeconds :type Float%20%28single-precision%29))
  (bind _firstplayer (Class|BPIGameMode|GetPlayerPos(Message) (Game|GetGameMode)))
  (Utilities|IsValid _firstplayer
    (:Is%20Valid
      (Development|PrintString (Utilities|String|ToString(Vector) (Transformation|GetActorLocation _firstplayer)) true true "(R=0.000000,G=0.660000,B=1.000000,A=1.000000)" DeltaSeconds)
      (if (< (.Z (Math|Vector|BreakVector (Transformation|GetActorLocation _firstplayer))) (Variables|Default|GetThreshold))
        (CallFunction|GenBatch)))))

(fn ConstructionScript
  (if (Variables|Default|GetResetNoise)
    (CallFunction|GenNoise)
    (Variables|Default|SetResetNoise false)))

(fn CreateMap
  (bind _size (Variables|Default|GetSize))
  (bind (_x _y) (Math|Vector2D|BreakVector2D _size))
  (for _index (range 0 (Math|Float|Truncate _y))
    (bind _output_get (Variables|Default|SetIndexY _index))
    (CallFunction|LineGen (Math|Float|Truncate _x) _output_get)))

(fn GenNoise
  (bind _returnvalue (Game|ConstructObjectfromClass "/Script/FastNoiseGenerator.FastNoiseWrapper"))
  (bind _output_get (Variables|Default|SetNoise _returnvalue))
  (Class|FastNoiseWrapper|SetupFastNoise _output_get "Perlin" (Math|Random|RandomIntegerinRange 0 50000) (Variables|/Game/Blueprint/DA_WorldGen.DA_WorldGen_C|GetNoiseFrequency (Variables|Default|GetWorldData)) "Quintic" "FBM" 3 1e+01 0.5 0.45 "Euclidean" "CellValue"))

(fn SpawnBloc
  (params (BlockClass :type Bp%20Dig%20Block%20Class%20Reference) (Index :type Vector%202D%20Structure))
  (bind (_x _y) (Math|Vector2D|BreakVector2D Index))
  (Game|SpawnActorfromClass BlockClass (Math|Transform|MakeTransform (+ (Transformation|GetActorLocation) (Math|Vector|MakeVector 0.0 (* _x 2e+02) (* _y -2e+02))) (Math|Rotator|MakeRotator 0.0 0.0 (Math|Conversions|ToFloat(Integer) (* (Math|Float|Round (* (Math|Random|RandomFloat) 4.0)) 90)))) "Undefined" "MultiplyWithRoot" 0 0))

(fn LineMultValue
  (params (Value :type Float%20%28double-precision%29) (Line :type Integer) (Intensity :type Float%20%28double-precision%29))
  (return (- Value (Math|Float|Clamp(Float) (* Line Intensity) 0.0 0.2))))

(fn GenBatch
  (for _index (range (Variables|Default|GetIndexY) (+ (Variables|Default|GetIndexY) 20))
    (CallFunction|LineGen (Math|Float|Truncate (.X (Math|Vector2D|BreakVector2D (Variables|Default|GetSize)))) _index))
  (Variables|Default|SetThreshold (- (Variables|Default|GetThreshold) 4e+03))
  (Variables|Default|SetIndexY (+ (Variables|Default|GetIndexY) 20)))

(fn LineGen
  (params (InputPin :type Integer) (IndexY :type Integer))
  (bind _worlddata (Variables|Default|GetWorldData))
  (LocalVariables|SetIndexLine IndexY)
  (for _index (range 0 InputPin)
    (if (<= (LocalVariables|GetIndexLine) 2)
      (CallFunction|SpawnBloc "/Game/Blueprint/BP_Mud.BP_Mud_C" (Math|Vector2D|MakeVector2D (Math|Conversions|ToFloat(Integer) _index) (Math|Conversions|ToFloat(Integer) (LocalVariables|GetIndexLine))))
      (elif (>= (+ (* (Math|Float|Clamp(Float) (Class|FastNoiseWrapper|GetNoise2D (Variables|Default|GetNoise) (Math|Conversions|ToFloat(Integer) _index) (Math|Conversions|ToFloat(Integer) (LocalVariables|GetIndexLine)))) (Variables|/Game/Blueprint/DA_WorldGen.DA_WorldGen_C|GetHardness _worlddata)) (* (Math|Random|RandomFloat) (Variables|/Game/Blueprint/DA_WorldGen.DA_WorldGen_C|GetRandomValueInBlockGen _worlddata))) (CallFunction|LineMultValue (Variables|/Game/Blueprint/DA_WorldGen.DA_WorldGen_C|GetRockAmount _worlddata) (LocalVariables|GetIndexLine) (Variables|/Game/Blueprint/DA_WorldGen.DA_WorldGen_C|GetRockIncreaseIntensity _worlddata)))
        (CallFunction|SpawnBloc "/Game/Blueprint/BP_Rock.BP_Rock_C" (Math|Vector2D|MakeVector2D (Math|Conversions|ToFloat(Integer) _index) (Math|Conversions|ToFloat(Integer) (LocalVariables|GetIndexLine))))
        (elif (>= (+ (* (Math|Float|Clamp(Float) (Class|FastNoiseWrapper|GetNoise2D (Variables|Default|GetNoise) (Math|Conversions|ToFloat(Integer) _index) (Math|Conversions|ToFloat(Integer) (LocalVariables|GetIndexLine)))) (Variables|/Game/Blueprint/DA_WorldGen.DA_WorldGen_C|GetHardness _worlddata)) (* (Math|Random|RandomFloat) (Variables|/Game/Blueprint/DA_WorldGen.DA_WorldGen_C|GetRandomValueInBlockGen _worlddata))) (CallFunction|LineMultValue (Variables|/Game/Blueprint/DA_WorldGen.DA_WorldGen_C|GetGravelAmount _worlddata) (LocalVariables|GetIndexLine) (Variables|/Game/Blueprint/DA_WorldGen.DA_WorldGen_C|GetGravelIncreaseIntensity _worlddata)))
          (CallFunction|SpawnBloc "/Game/Blueprint/BP_Gravel.BP_Gravel_C" (Math|Vector2D|MakeVector2D (Math|Conversions|ToFloat(Integer) _index) (Math|Conversions|ToFloat(Integer) (LocalVariables|GetIndexLine))))
          (elif (not (<= (+ (* (Math|Float|Clamp(Float) (Class|FastNoiseWrapper|GetNoise2D (Variables|Default|GetNoise) (Math|Conversions|ToFloat(Integer) _index) (Math|Conversions|ToFloat(Integer) (LocalVariables|GetIndexLine)))) (Variables|/Game/Blueprint/DA_WorldGen.DA_WorldGen_C|GetHardness _worlddata)) (* (Math|Random|RandomFloat) (Variables|/Game/Blueprint/DA_WorldGen.DA_WorldGen_C|GetRandomValueInBlockGen _worlddata))) (Variables|/Game/Blueprint/DA_WorldGen.DA_WorldGen_C|GetCaveAmount _worlddata)))
            (CallFunction|SpawnBloc "/Game/Blueprint/BP_Mud.BP_Mud_C" (Math|Vector2D|MakeVector2D (Math|Conversions|ToFloat(Integer) _index) (Math|Conversions|ToFloat(Integer) (LocalVariables|GetIndexLine))))))))))

(fn BonusBlock)