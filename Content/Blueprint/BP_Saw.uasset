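; BP_Saw is a saw hazard that reports overlaps to its parent BP_Camera to check for player death.
; On overlap, it casts its parent actor to BP_Camera and passes the overlapping actor to CheckPlayerDeath.
; Each tick it teleport-free moves down in world Z by OffsetDown without sweeping, then multiplies that offset by LerpSpeed, so the step scales geometrically per frame, independent of delta time.
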(event EventBeginPlay)

(event Collision|EventActorBeginOverlap
  (params (OtherActor :type Actor%20Object%20Reference))
  (bind _asbp_camera (Utilities|Casting|CastToBP_Camera (Actor|GetParentActor)))
  (Default|CheckPlayerDeath _asbp_camera OtherActor))

(event EventTick
  (params (DeltaSeconds :type Float%20%28single-precision%29))
  (bind _returnvalue (Transformation|GetActorLocation))
  (Transformation|SetActorLocation (Math|Vector|MakeVector (.x _returnvalue) (.y _returnvalue) (- (.z _returnvalue) (Variables|Default|GetOffsetDown))) false false)
  (Variables|Default|SetOffsetDown (* (Variables|Default|GetOffsetDown) (Variables|Default|GetLerpSpeed))))

(fn ConstructionScript)