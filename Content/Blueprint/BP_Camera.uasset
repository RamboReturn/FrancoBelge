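; BP_Camera is a shared two-player camera that follows a downward race and ends the round when a player falls behind.
; Each tick it finds the lower character as leader and eases its Z down toward that height plus an adjustable offset, never moving back up.
; When the higher character's vertical distance from the camera exceeds a threshold, it shows the end-round widget and switches input to UI only.
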(event EventBeginPlay
  (Variables|Default|SetbFindCameraComponentWhenViewTarget true)
  (Game|Player|SetViewTargetwithBlend (Game|GetPlayerController 0) self 0.0 "VTBlend_Linear" 0.0 false))

(event Collision|EventActorBeginOverlap
  (params (OtherActor :type Actor%20Object%20Reference)))

(event EventTick
  (params (DeltaSeconds :type Float%20%28single-precision%29))
  (bind (_first_player_pos _lastplayer) (CallFunction|CheckWhichPlayerIsBottom))
  (CallFunction|UpdateCamPos _first_player_pos)
  (CallFunction|CheckPlayerDeath _lastplayer))

(fn ConstructionScript)

(fn UpdateCamPos
  (params (First%20Player%20Pos :type Vector))
  (bind _returnvalue (Transformation|GetActorLocation))
  (bind _z (Math|Vector|BreakVector First%20Player%20Pos))
  (bind _returnvalue_2 (Transformation|GetActorLocation))
  (bind _offsetcamz (Variables|Default|GetoffsetCamZ))
  (bind _z_2 (Math|Vector|BreakVector _returnvalue_2))
  (bind _returnvalue_3 (Math|Float|Lerp -7e+02 7e+02 _offsetcamz))
  (bind _returnvalue_4 (+ _z _returnvalue_3))
  (Math|Float|CompareFloat _z_2 _returnvalue_4
    (:>
      (bind _output_get (Variables|Default|SettargetCamPos (Math|Vector|MakeVector (.x _returnvalue) (.y _returnvalue) (Math|Interpolation|FInterpTo _z_2 _returnvalue_4 (Utilities|Time|GetWorldDeltaSeconds) (Math|Float|Lerp 2.0 1.0 (Math|Float|NormalizetoRange (- _z_2 _returnvalue_4) 0.0 1e+03))))))
      (Transformation|SetActorLocation _output_get true false)
      (return))))

(fn CheckPlayerDeath
  (params (Last%20Player :type Actor%20Object%20Reference))
  (Math|Float|CompareFloat (Class|Actor|GetVerticalDistanceto Last%20Player) 1.35e+03
    (:>
      (bind _returnvalue (UserInterface|CreateWidget "/Game/UI/EndRoundUI.EndRoundUI_C"))
      (UserInterface|Viewport|AddtoViewport _returnvalue 0)
      (Input|SetInputModeUIOnly (Game|GetPlayerController 0) 0 "DoNotLock" false))))

(fn CheckWhichPlayerIsBottom
  (bind _outactors (Actor|GetAllActorsOfClass "/Game/Blueprint/BP_ThirdPersonCharacter.BP_ThirdPersonCharacter_C"))
  (Math|Float|CompareFloat (.Z (Math|Vector|BreakVector (Transformation|GetActorLocation (Utilities|Array|Get(acopy) _outactors)))) (.Z (Math|Vector|BreakVector (Transformation|GetActorLocation (Utilities|Array|Get(acopy) _outactors 1))))
    (:>
      (return (Math|Conversions|ToVector(Float) (.Z (Math|Vector|BreakVector (Transformation|GetActorLocation (Utilities|Array|Get(acopy) _outactors 1))))) (Utilities|Array|Get(acopy) _outactors)))
    (:<
      (return (Transformation|GetActorLocation (Utilities|Array|Get(acopy) _outactors)) (Utilities|Array|Get(acopy) _outactors 1)))))