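; BP_voxeltype is an actor that pairs a static mesh component named Fan with a configurable, voxel-themed Niagara effect.
; The construction script assigns the chosen mesh to Fan, then passes a texture, grid size and voxel count to the Niagara component as user parameters.
; All setup happens at construction, and the event graph holds only disabled placeholder events.
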(event EventBeginPlay)

(event Collision|EventActorBeginOverlap
  (params (OtherActor :type Actor%20Object%20Reference)))

(event EventTick
  (params (DeltaSeconds :type Float%20%28single-precision%29)))

(fn ConstructionScript
  (bind _niagara (Variables|Default|GetNiagara))
  (Components|StaticMesh|SetStaticMesh (Variables|Default|GetFan) (Variables|Default|GetStaticMesh))
  (Niagara|SetTextureObject (Variables|Default|GetNiagara) "Texture" (Variables|Default|GetTexture))
  (Effects|Components|ParticleSystem|SetFloatParameter _niagara "GridSize" (Variables|Default|Get_GridSize))
  (Effects|Components|ParticleSystem|SetFloatParameter _niagara "VoxelCount" (Math|Conversions|ToFloat(Integer) (Variables|Default|Get_VoxelCount))))